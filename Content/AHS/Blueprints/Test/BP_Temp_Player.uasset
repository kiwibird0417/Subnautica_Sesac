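; Temporary test player pawn for underwater movement, tracking depth and oxygen and showing a temp UI widget.
; Each tick derives a scaled depth from a Surface reference and drains oxygen below it, refilling instantly to max above.
; Left click runs a debug-drawn sphere trace around the pawn, matching the hit actor's display name to set movement speed ("Speed") or oxygen drain rate ("Tank").
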(event EventBeginPlay
  (bind _returnvalue (UserInterface|CreateWidget "/Game/AHS/Blueprints/UI/WBP_TempUI.WBP_TempUI_C"))
  (UserInterface|Viewport|AddtoViewport _returnvalue 0))

(event Collision|EventActorBeginOverlap
  (params (OtherActor :type Actor%20Object%20Reference)))

(event EventTick
  (params (DeltaSeconds :type Float%20%28single-precision%29))
  (CallFunction|CurrentDepthUI)
  (CallFunction|OxygenTimer DeltaSeconds))

(event Input|MouseEvents|LeftMouseButton
  (params (Key :type Key%20Structure :default "None"))
  (bind _returnvalue (Transformation|GetActorLocation))
  (:Pressed
    (bind _outhit (Collision|SphereTraceForObjects _returnvalue _returnvalue 2e+02 (Variables|Default|GetObject%20Types) false 0 "ForDuration"))
    (if (Utilities|String|Contains (Utilities|GetDisplayName (.hitactor _outhit)) "Speed")
      (Variables|/Script/Engine.FloatingPawnMovement|SetMaxSpeed (Variables|Default|GetFloatingPawnMovement) 2e+02)
      (elif (Utilities|String|Contains (Utilities|GetDisplayName (.hitactor _outhit)) "Tank")
        (Variables|Default|SetOxygenDecreaseRate 1.0)))))

(fn ConstructionScript)

(fn CurrentDepthUI
  (Variables|Default|SetCurrent_PlayerDepth (Class|KismetMathLibrary|ToInt64(Float) (* (.z (- (Variables|Default|GetSurface) (Transformation|GetActorLocation))) 0.05))))

(fn OxygenTimer
  (params (DeltaSeconds :type Float%20%28double-precision%29))
  (bind _oxygendecreaserate (Variables|Default|GetOxygenDecreaseRate))
  (if (< (.z (Transformation|GetActorLocation)) (.z (Variables|Default|GetSurface)))
    (Variables|Default|SetbIsUnderwater true)
    (if (not (<= (Variables|Default|GetOxygen) 0.0))
      (Variables|Default|SetOxygen (- (Variables|Default|GetOxygen) (* _oxygendecreaserate (Utilities|Time|GetWorldDeltaSeconds))))
      (Development|PrintString (Utilities|String|ToString(Float) _oxygendecreaserate)))
    (else
      (Variables|Default|SetbIsUnderwater false)
      (Variables|Default|SetOxygen (Variables|Default|GetMaxOxygen)))))